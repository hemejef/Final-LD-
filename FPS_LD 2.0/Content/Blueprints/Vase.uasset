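; Vase is a breakable prop that adds to the player's destruction tally when hit.
; On Hit it casts the other actor to Melee, Shooter2 or DestroyableGlass, and increments ThingsDestroyed on FirstPersonCharacterTrue before destroying itself.
; Melee and Shooter2 actors are destroyed along with the vase, while DestroyableGlass survives the impact.
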(event `self.ReceiveHit`
  (params (MyComp :type "PrimitiveComponent Object Reference") (Other :type "Actor Object Reference") (OtherComp :type "PrimitiveComponent Object Reference") (bSelfMoved :type Boolean) (HitLocation :type "Vector Structure") (HitNormal :type "Vector Structure") (NormalImpulse :type "Vector Structure") (Hit :type "HitResult Structure (by ref)"))
  (bind _returnvalue (`GameplayStatics.GetPlayerCharacter` 0))
  (cast `/Game/Blueprints/AI/Melee` Other
    (:`then`
      (`KismetSystemLibrary.PrintString` "hit melee")
      (bind _asfirst_person_character_true (cast `/Game/FirstPersonBP/Blueprints/FirstPersonCharacterTrue` _returnvalue :!label _label))
      (`/Engine/EditorBlueprintResources/StandardMacros.IncrementInt` (`/Game/FirstPersonBP/Blueprints/FirstPersonCharacterTrue.ThingsDestroyed` _asfirst_person_character_true)
        (:`  `
          (`self.K2_DestroyActor` Other))))
    (:`CastFailed`
      (cast `/Game/Blueprints/AI/shooter2` Other
        (:`then`
          (goto _label))
        (:`CastFailed`
          (cast `/Game/Blueprints/DestroyableGlass` Other)
          (bind _asfirst_person_character_true_2 (cast `/Game/FirstPersonBP/Blueprints/FirstPersonCharacterTrue` _returnvalue))
          (`/Engine/EditorBlueprintResources/StandardMacros.IncrementInt` (`/Game/FirstPersonBP/Blueprints/FirstPersonCharacterTrue.ThingsDestroyed` _asfirst_person_character_true_2)
            (:`  `
              _))))))
  (`self.K2_DestroyActor`))

(event `ReceiveBeginPlay_Copy`)

(event `self.ReceiveBeginPlay`)

(event `ReceiveTick_Copy`
  (params (DeltaSeconds :type "Float (double-precision)" :default 0.0)))

(event `self.ReceiveTick`
  (params (DeltaSeconds :type "Float (single-precision)")))

(fn `UserConstructionScript`)