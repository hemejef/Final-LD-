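; Destroyable glass actor that reacts when a Bottle, Vase or Statue hits its Destructible component.
; On such a hit it applies point damage to the hit actor, with the striking object as damage causer.
; All three cast branches then increment the player character's ThingsDestroyed counter and destroy the glass actor after a short delay.
; The counter has no guard against repeated hits during that delay.
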(event `self.Destructible.OnComponentHit`
  (params (OtherActor :type "Actor Object Reference") (OtherComp :type "PrimitiveComponent Object Reference") (NormalImpulse :type "Vector Structure") (Hit :type "HitResult Structure (by ref)"))
  (bind (_bblockinghit _binitialoverlap _time _location _impactpoint _normal _impactnormal _physmat _hitactor) (`GameplayStatics.BreakHitResult` Hit))
  (bind _asbottle (cast `/Game/Blueprints/Bottle` OtherActor)
    (:`then`
      (`GameplayStatics.ApplyPointDamage` _hitactor 0.0 _impactpoint Hit null _asbottle))
    (:`CastFailed`
      (bind _asvase (cast `/Game/Blueprints/Vase` OtherActor)
        (:`then`
          (`GameplayStatics.ApplyPointDamage` _hitactor 0.0 _impactpoint Hit null _asvase))
        (:`CastFailed`
          (bind _asstatue (cast `/Game/Blueprints/Statue` OtherActor))
          (`GameplayStatics.ApplyPointDamage` _hitactor 0.0 _impactpoint Hit null _asstatue)))))
  (bind _asfirst_person_character_true (cast `/Game/FirstPersonBP/Blueprints/FirstPersonCharacterTrue` (`GameplayStatics.GetPlayerCharacter` 0)))
  (`/Engine/EditorBlueprintResources/StandardMacros.IncrementInt` (`/Game/FirstPersonBP/Blueprints/FirstPersonCharacterTrue.ThingsDestroyed` _asfirst_person_character_true)
    (:`  `
      (`KismetSystemLibrary.Delay` 4.0)
      (`self.K2_DestroyActor`))))

(event `self.ReceiveBeginPlay`)

(event `self.ReceiveActorBeginOverlap`
  (params (OtherActor :type "Actor Object Reference")))

(event `self.ReceiveTick`
  (params (DeltaSeconds :type "Float (single-precision)")))

(fn `UserConstructionScript`)